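; Enemy turret Blueprint that aims and fires at a sensed TopDownCharacter and can be destroyed by damage.
; When PawnSensing sees the character, the Turret component turns via a look-at rotation set as relative rotation.
; It spawns Player_projectile_BP at BulletSpawnLocation, throttled by a boolean and Delay cooldown.
; Damage reduces health initialized from MaxHp, destroying the actor at zero; an impulse node is left unconnected.
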(event OnSeePawn(PawnSensing)
  (params (Pawn :type Pawn%20Object%20Reference))
  (bind _astop_down_character (Utilities|Casting|CastToTopDownCharacter Pawn))
  (Utilities|FlowControl|Sequence
    (:then_0
      (Transformation|SetRelativeRotation (Variables|Default|GetTurret) (Math|Rotator|FindLookatRotation (Transformation|GetActorLocation) (Transformation|GetActorLocation _astop_down_character)) false false))
    (:then_1
      (if (Variables|Default|GetSpawnProjectile)
        (Game|SpawnActorfromClass "/Game/Blueprints/Player_projectile_BP.Player_projectile_BP_C" (Transformation|GetWorldTransform (Variables|Default|GetBulletSpawnLocation)) "Undefined" 0 0)
        (Variables|Default|SetSpawnProjectile false)
        (Utilities|FlowControl|Delay 1.5)
        (Variables|Default|SetSpawnProjectile true)))))

(event Game|Damage|EventAnyDamage
  (params (Damage :type Float%20%28single-precision%29) (DamageType :type Damage%20Type%20Object%20Reference) (InstigatedBy :type Controller%20Object%20Reference) (DamageCauser :type Actor%20Object%20Reference))
  (bind _output_get (Variables|Default|SetCurrentHp (- (Variables|Default|GetCurrentHp) Damage)))
  (if (<= _output_get 0.0)
    (Actor|DestroyActor)))

(event EventBeginPlay
  (Variables|Default|SetCurrentHp (Variables|Default|GetMaxHp)))

(fn ConstructionScript)