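; Enemy drone that patrols at random, shoots at the player on sight and is destroyed when damage depletes its health.
; Patrol loops AIMoveTo to random nearby navigable points with a pause between moves, and stops re-queuing once SeePlayer is set, which is never cleared.
; PawnSensing turns the drone toward the TopDownCharacter and fires impulse-launched projectiles, throttled by a boolean and Delay cooldown.
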(event OnSeePawn(PawnSensing)
  (params (Pawn :type Pawn%20Object%20Reference))
  ;[1 1 1] Look at and Shoot at pawn
  (Variables|Default|SetSeePlayer true)
  (bind _astop_down_character (Utilities|Casting|CastToTopDownCharacter Pawn))
  (Utilities|FlowControl|Sequence
    (:then_0
      (Transformation|SetActorRotation (Math|Rotator|FindLookatRotation (Transformation|GetActorLocation) (Transformation|GetActorLocation _astop_down_character))))
    (:then_1
      (if (Variables|Default|GetSpawnProjectile)
        (bind _returnvalue (Game|SpawnActorfromClass "/Game/Enemies/Blueprints/FirstPersonProjectile.FirstPersonProjectile_C" (Transformation|GetWorldTransform (Variables|Default|GetBulletSpawnLocation)) "Undefined" 0 0))
        (Physics|AddImpulse (Variables|/Game/Enemies/Blueprints/FirstPersonProjectile.FirstPersonProjectile_C|GetSphere _returnvalue) (* (Math|Vector|GetForwardVector (Variables|Default|GetCube)) (Variables|Default|GetShootAmount)) "None" true)
        (Variables|Default|SetSpawnProjectile false)
        (Utilities|FlowControl|Delay 1.5)
        (Variables|Default|SetSpawnProjectile true)))))

(event Custom|MoveToRandomLocation
  ;[1 1 1] Move to random location (patrol)
  (if (not (Variables|Default|GetSeePlayer))
    (AI|AIMoveTo self (.RandomLocation (Class|NavigationSystemV1|GetRandomPointinNavigableRadius (Transformation|GetActorLocation) 5e+02 0 0)) 0 5.0 false
      (:OnSuccess
        (Utilities|FlowControl|Delay 1.5)
        (CallFunction|MovetoRandomLocation)))))

(event Game|Damage|EventAnyDamage
  (params (Damage :type Float%20%28single-precision%29) (DamageType :type Damage%20Type%20Object%20Reference) (InstigatedBy :type Controller%20Object%20Reference) (DamageCauser :type Actor%20Object%20Reference))
  (bind _output_get (Variables|Default|SetCurrentHp (- (Variables|Default|GetCurrentHp) Damage)))
  (if (<= _output_get 0.0)
    (Actor|DestroyActor)))

(event EventBeginPlay
  ;[1 1 1] Move to random location (patrol)
  (Variables|Default|SetCurrentHp (Variables|Default|GetMaxHp))
  (CallFunction|MovetoRandomLocation))

(fn ConstructionScript)