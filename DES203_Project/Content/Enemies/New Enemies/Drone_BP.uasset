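; Drone enemy that patrols at random and shoots at the player when it spots them.
; PawnSensing sets a spotted flag that clears after a delay.
; Tick either turns the drone toward the seen TopDownCharacter and fires, or, once the last move succeeds, sends it via AIMoveTo to a random reachable point.
; FireWeapon runs every tick while spotted, with a Delay throttling spawns of Player_projectile_BP at BulletSpawn1.
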(event OnSeePawn(PawnSensing)
  (params (Pawn :type Pawn%20Object%20Reference))
  ;[1 1 1] Player Detection
  (Variables|Default|SetTargetSpotted? true)
  (Utilities|FlowControl|Delay 5.0)
  (Variables|Default|SetTargetSpotted? false))

(event Custom|Fire%20Weapon
  ;[1 1 1] Projectile Spawning
  (Utilities|FlowControl|Delay 0.75)
  (Game|SpawnActorfromClass "/Game/Blueprints/Player_projectile_BP.Player_projectile_BP_C" (Transformation|GetWorldTransform (Variables|Default|GetBulletSpawn1)) "Undefined" 0 0))

(event EventBeginPlay)

(event Collision|EventActorBeginOverlap
  (params (OtherActor :type Actor%20Object%20Reference)))

(event EventTick
  (params (DeltaSeconds :type Float%20%28single-precision%29))
  ;[1 1 1] Patrol
  (if (Variables|Default|GetTargetSpotted?)
    ;[1 1 1] Player Detected
    (Development|PrintString "Detect")
    (bind _astop_down_character (Utilities|Casting|CastToTopDownCharacter (stale OnSeePawn(PawnSensing) Pawn)))
    (Utilities|FlowControl|Sequence
      (:then_0
        (Transformation|SetActorRotation (Math|Rotator|FindLookatRotation (Transformation|GetActorLocation) (Transformation|GetActorLocation _astop_down_character)))
        (CallFunction|FireWeapon)))
    (elif (Variables|Default|GetTargetReached?)
      (Development|PrintString "No Detect")
      (AI|AIMoveTo self (.RandomLocation (AI|Navigation|GetRandomReachablePointinRadius (Transformation|GetWorldLocation (Variables|Default|GetBody)) 5e+03 0 0)) 0 1.0 false
        (:then
          (Variables|Default|SetTargetReached? false))
        (:OnSuccess
          (Variables|Default|SetTargetReached? true))))))

(fn ConstructionScript)