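; Test AI drone Blueprint that patrols random reachable points, shoots at spotted players and explodes when its health runs out.
; PawnSensing sets a spotted flag, cleared after a delay, which Tick uses to choose between attacking and wandering via AIMoveTo.
; Attacking turns the drone toward the TopDownCharacter and calls FireWeapon every tick, with a Delay pacing projectile spawns.
; Damage reduces health until an explosion plays and the actor is destroyed shortly after.
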(event OnSeePawn(PawnSensing)
  (params (Pawn :type Pawn%20Object%20Reference))
  ;[1 1 1] Player Detection
  (Variables|Default|SetTargetSpotted? true)
  (Utilities|FlowControl|Delay 5.0)
  (Variables|Default|SetTargetSpotted? false))

(event Custom|Fire%20Weapon
  ;[1 1 1] Projectile Spawning
  (Utilities|FlowControl|Delay 0.75)
  (Game|SpawnActorfromClass "/Game/Enemies/Blueprints/FirstPersonProjectile.FirstPersonProjectile_C" (Transformation|GetWorldTransform (Variables|Default|GetBulletSpawn1)) "Undefined" 0 0))

(event EventBeginPlay
  (Variables|Default|SetCurrentHp (Variables|Default|GetMaxHp)))

(event Collision|EventActorBeginOverlap
  (params (OtherActor :type Actor%20Object%20Reference)))

(event EventTick
  (params (DeltaSeconds :type Float%20%28single-precision%29))
  ;[1 1 1] Patrol
  (if (Variables|Default|GetTargetSpotted?)
    ;[1 1 1] Player Detected
    (bind _astop_down_character (Utilities|Casting|CastToTopDownCharacter (stale OnSeePawn(PawnSensing) Pawn)))
    (Utilities|FlowControl|Sequence
      (:then_0
        (Transformation|SetActorRotation (Math|Rotator|FindLookatRotation (Transformation|GetActorLocation) (Transformation|GetActorLocation _astop_down_character)))
        (CallFunction|FireWeapon)))
    (elif (Variables|Default|GetTargetReached?)
      (AI|AIMoveTo self (.RandomLocation (AI|Navigation|GetRandomReachablePointinRadius (Transformation|GetWorldLocation (Variables|Default|GetBody)) 5e+03 0 0)) 0 1.0 false
        (:then
          (Variables|Default|SetTargetReached? false))
        (:OnSuccess
          (Variables|Default|SetTargetReached? true))))))

(event Game|Damage|EventAnyDamage
  (params (Damage :type Float%20%28single-precision%29) (DamageType :type Damage%20Type%20Object%20Reference) (InstigatedBy :type Controller%20Object%20Reference) (DamageCauser :type Actor%20Object%20Reference))
  (bind _capsulecomponent (Variables|Collision|GetCapsuleComponent))
  (bind _output_get (Variables|Default|SetCurrentHp (- (Variables|Default|GetCurrentHp) Damage)))
  (if (<= _output_get 0.0)
    (Rendering|SetVisibility _capsulecomponent false false)
    (Effects|SpawnEmitteratLocation "/Game/StarterContent/Particles/P_Explosion.P_Explosion" (Transformation|GetWorldLocation _capsulecomponent))
    (Utilities|FlowControl|Delay 1.0)
    (Actor|DestroyActor)))

(fn ConstructionScript)