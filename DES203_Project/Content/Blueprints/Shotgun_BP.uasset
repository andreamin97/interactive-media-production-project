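; Shotgun weapon Blueprint that fires a fan of Player_projectile_BP actors when its Shoot event runs.
; Shoot swings ShootArrow0 back, then loops, spawning a projectile at the arrow's transform (skipped if colliding) and stepping its rotation, with a Delay inside the loop.
; It then spawns a muzzle effect at AimArrow and a sound at the world origin.
; An older chain of always-spawn projectile calls is left unconnected.
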(event EventBeginPlay)

(event Collision|EventActorBeginOverlap
  (params (OtherActor :type Actor%20Object%20Reference)))

(event EventTick
  (params (DeltaSeconds :type Float%20%28single-precision%29)))

(event EventShoot
  (bind _aimarrow (Variables|Default|GetaimArrow))
  (Transformation|AddRelativeRotation (Variables|Default|GetShootArrow_0) "0,-60.000000, 0" false false)
  (for _index (range 0 5)
    (Game|SpawnActorfromClass "/Game/Blueprints/Player_projectile_BP.Player_projectile_BP_C" (Transformation|GetWorldTransform (Variables|Default|GetShootArrow_0)) "DontSpawnIfColliding" 0 0)
    (Transformation|AddRelativeRotation (Variables|Default|GetShootArrow_0) "0,10.000000, 0" false false)
    (Utilities|FlowControl|Delay 1.0))
  (Effects|SpawnEmitteratLocation (Variables|Default|GetshootEffect) (Transformation|GetWorldLocation _aimarrow) (Transformation|GetWorldRotation _aimarrow) "2.000000,2.000000,2.000000")
  (Audio|SpawnSoundatLocation (Variables|Default|GetShootSFX) "0, 0, 0" "0, 0, 0" 1.0 1.0 0.0 0 0))

(fn ConstructionScript
  (|CallParentFunction))