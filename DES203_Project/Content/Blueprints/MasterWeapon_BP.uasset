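; Base weapon Blueprint that fires player projectiles and carries a laser pointer.
; The Shoot event spawns a Player_projectile_BP at the AimArrow transform, with a muzzle effect and sound at the same point.
; The laser pointer function sets the particle LaserRange parameter slightly short of Range; its hit-distance branch is disconnected, so Distance and HasHit have no effect.
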(event EventShoot
  (bind _aimarrow (Variables|Default|GetaimArrow))
  (bind _aimarrow_2 (Variables|Default|GetaimArrow))
  (bind _returnvalue (Transformation|GetWorldTransform _aimarrow))
  (bind _returnvalue_2 (Transformation|GetWorldLocation _aimarrow_2))
  (Game|SpawnActorfromClass "/Game/Blueprints/Player_projectile_BP.Player_projectile_BP_C" (Math|Transform|MakeTransform (.location _returnvalue) (.rotation _returnvalue) "1,1,1") "AlwaysSpawn" 0 0)
  (Effects|SpawnEmitteratLocation (Variables|Default|GetshootEffect) _returnvalue_2 (Transformation|GetWorldRotation _aimarrow_2))
  (Audio|SpawnSoundatLocation (Variables|Default|GetShootSFX) _returnvalue_2 "0, 0, 0" 1.0 1.0 0.0 0 0))

(fn ConstructionScript)

(fn SetLaserPointerFunction
  (params (Distance :type Float%20%28single-precision%29) (HasHit :type Boolean))
  (Effects|Components|ParticleSystem|SetVectorParameter (Variables|Default|GetlaserPointer) "LaserRange" (Math|Vector|MakeVector (- (Variables|Default|Getrange) 5e+01) 0.0 0.0)))