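; Rifle weapon Blueprint with a shoot action and a laser pointer.
; Shoot spawns an old-version player projectile at the AimArrow transform, always spawning despite collisions, and plays a shoot effect there.
; The laser pointer function sets the emitter's LaserRange vector parameter to slightly short of the weapon's Range.
; Its branch for shortening the laser to a hit distance is disconnected, so both inputs are ignored.
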(event EventShoot
  (bind _aimarrow (Variables|Default|GetaimArrow))
  (Game|SpawnActorfromClass "/Game/Blueprints/oldweapons/Blueprints/Player_projectile_BP_OLD.Player_projectile_BP_OLD_C" (Transformation|GetWorldTransform (Variables|Default|GetaimArrow)) "AlwaysSpawn" 0 0)
  (Effects|SpawnEmitteratLocation (Variables|Default|GetshootEffect) (Transformation|GetWorldLocation _aimarrow) (Transformation|GetWorldRotation _aimarrow)))

(fn ConstructionScript)

(fn SetLaserPointerFunction
  (params (Distance :type Float%20%28single-precision%29) (HasHit :type Boolean))
  (Effects|Components|ParticleSystem|SetVectorParameter (Variables|Default|GetlaserPointer) "LaserRange" (Math|Vector|MakeVector (- (Variables|Default|Getrange) 5e+01) 0.0 0.0)))