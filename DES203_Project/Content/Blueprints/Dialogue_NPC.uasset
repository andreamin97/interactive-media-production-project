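; Dialogue NPC that shows a dialogue widget while the TopDownCharacter is inside its Cylinder trigger.
; Entering sets ActiveTextLine to the first DialogueText entry, and leaving hides the widget.
; The Continue input steps ActiveTextLine through the array, stopping at the last entry.
; DialogIndex is not reset on re-entry, and Continue does not check for overlap.
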(event OnComponentBeginOverlap(Cylinder)
  (params (OverlappedComponent :type Primitive%20Component%20Object%20Reference) (OtherActor :type Actor%20Object%20Reference) (OtherComp :type Primitive%20Component%20Object%20Reference) (OtherBodyIndex :type Integer) (bFromSweep :type Boolean) (SweepResult :type Hit%20Result%20Structure%20%28by%20ref%29))
  (Utilities|Casting|CastToTopDownCharacter OtherActor)
  (Rendering|SetVisibility (Variables|Default|GetWidget) true false)
  (Variables|Default|SetActiveTextLine (Utilities|Array|Get(acopy) (Variables|Default|GetDialogueText))))

(event OnComponentEndOverlap(Cylinder)
  (params (OverlappedComponent :type Primitive%20Component%20Object%20Reference) (OtherActor :type Actor%20Object%20Reference) (OtherComp :type Primitive%20Component%20Object%20Reference) (OtherBodyIndex :type Integer))
  (Utilities|Casting|CastToTopDownCharacter OtherActor)
  (Rendering|SetVisibility (Variables|Default|GetWidget) false false))

(event EventBeginPlay)

(event Collision|EventActorBeginOverlap
  (params (OtherActor :type Actor%20Object%20Reference)))

(event EventTick
  (params (DeltaSeconds :type Float%20%28single-precision%29)))

(event Input|ActionEvents|InputActionContinue
  (params (Key :type Key%20Structure :default "None"))
  (:Pressed
    (if (not (>= (+ (Variables|Default|GetDialogIndex) 1) (Utilities|Array|Length (Variables|Default|GetDialogueText))))
      (bind _output_get (Variables|Default|SetDialogIndex (+ (Variables|Default|GetDialogIndex) 1)))
      (Variables|Default|SetActiveTextLine (Utilities|Array|Get(acopy) (Variables|Default|GetDialogueText) _output_get)))))

(fn ConstructionScript)