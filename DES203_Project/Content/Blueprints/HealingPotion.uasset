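; Healing potion with limited charges that restores the player's health gradually when used.
; Use spends a charge and starts a fast looping timer, unless a heal is already running.
; Each Heal tick applies negative damage to player pawn 0 and counts down the Healing pool.
; Once the pool is empty, the timer is cleared and the pool resets for the next use.
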(event Custom|Heal
  (if (> (Variables|Default|GetHealing) 0.0)
    (Game|Damage|ApplyDamage (Game|Player|GetPlayerPawn 0) -1.0 0 0)
    (Variables|Default|SetHealing (- (Variables|Default|GetHealing) 1.0))
    (else
      (Utilities|Time|ClearandInvalidateTimerbyHandle (Variables|Default|GetHealTimer))
      (Variables|Default|SetHealing 5.0))))

(event EventBeginPlay)

(event Collision|EventActorBeginOverlap
  (params (OtherActor :type Actor%20Object%20Reference)))

(event EventTick
  (params (DeltaSeconds :type Float%20%28single-precision%29)))

(event EventUse
  (if (> (Variables|Default|Getcharges) 0)
    (if (not (Class|KismetSystemLibrary|TimerExistsHandle (Variables|Default|GetHealTimer)))
      (Variables|Default|Setcharges (- (Variables|Default|Getcharges) 1))
      (bind _returnvalue (Utilities|Time|SetTimerbyEvent (delegate Custom|Heal) 0.15 true))
      (Variables|Default|SetHealTimer _returnvalue))))

(fn ConstructionScript)