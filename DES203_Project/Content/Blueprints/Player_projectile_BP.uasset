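; Player projectile for a top-down shooter that takes its damage, effects and behavior from the player's equipped main weapon.
; On BeginPlay it copies damage, AoE flag, tracer and hit effects, sets gravity, and times self-destruction from weapon range divided by a hardcoded constant.
; On hit it ignores TopDownCharacters and other player projectiles, otherwise applies radial or direct damage, plays impact sound and effect, and destroys itself.
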(event Custom|KillAfterTime
  (Actor|DestroyActor))

(event EventBeginPlay
  (bind _projectile (Variables|MyProjectile|GetProjectile))
  (bind _astop_down_character (Utilities|Casting|CastToTopDownCharacter (Game|GetPlayerCharacter 0)))
  (bind _asmaster_weapon_bp (Utilities|Casting|CastToMasterWeapon_BP (Variables|/Script/DES203_Project.DES203_ProjectCharacter|GetMainWeapon _astop_down_character)))
  (Variables|Default|SetAoE (Variables|/Game/Blueprints/MasterWeapon_BP.MasterWeapon_BP_C|GetAoE _asmaster_weapon_bp))
  (Variables|Default|Setdamage (Variables|/Script/DES203_Project.RangedWeapon|Getdamage (Variables|/Script/DES203_Project.DES203_ProjectCharacter|GetMainWeapon _astop_down_character)))
  (Effects|Components|ParticleSystem|SetTemplate (Variables|Default|GetTracerVFX) (Variables|/Script/DES203_Project.RangedWeapon|GettracerEffect (Variables|/Script/DES203_Project.DES203_ProjectCharacter|GetMainWeapon _astop_down_character)))
  (Variables|Default|SethitVFX (Variables|/Script/DES203_Project.RangedWeapon|GetshootHit (Variables|/Script/DES203_Project.DES203_ProjectCharacter|GetMainWeapon _astop_down_character)))
  (if (Variables|/Game/Blueprints/MasterWeapon_BP.MasterWeapon_BP_C|GetusesGravity _asmaster_weapon_bp)
    (Variables|/Script/Engine.ProjectileMovementComponent|SetProjectileGravityScale _projectile 1.0)
    (else
      (Variables|/Script/Engine.ProjectileMovementComponent|SetProjectileGravityScale _projectile 0.0)))
  (if (Variables|/Game/Blueprints/MasterWeapon_BP.MasterWeapon_BP_C|GetHasDefined%20Range _asmaster_weapon_bp)
    (bind _returnvalue (Utilities|Time|SetTimerbyEvent (delegate Custom|KillAfterTime) (/ (Variables|/Script/DES203_Project.RangedWeapon|Getrange _asmaster_weapon_bp) 2e+03)))
    (Utilities|Time|UnpauseTimerbyHandle _returnvalue)))

(event Collision|EventHit
  (params (MyComp :type Primitive%20Component%20Object%20Reference) (Other :type Actor%20Object%20Reference) (OtherComp :type Primitive%20Component%20Object%20Reference) (bSelfMoved :type Boolean) (HitLocation :type Vector :default "0, 0, 0") (HitNormal :type Vector :default "0, 0, 0") (NormalImpulse :type Vector :default "0, 0, 0") (Hit :type Hit%20Result%20Structure%20%28by%20ref%29))
  (bind _damage (Variables|Default|Getdamage))
  ;[1 1 1] Apply damage
  (Utilities|Casting|CastToTopDownCharacter Other
    (:CastFailed
      (Utilities|Casting|CastToPlayer_projectile_BP Other
        (:CastFailed
          (if (Variables|Default|GetAoE)
            (Game|Damage|ApplyRadialDamage _damage HitLocation 3e+02 0 0 (Game|Player|GetPlayerPawn 0) 0 false "ECC_Visibility")
            (Audio|PlaySoundatLocation "/Game/PrototypeWeap/Sound/SniperRifle/SR_BulletImpact01.SR_BulletImpact01" HitLocation "0, 0, 0" 1.0 1.0 0.0 0 0 0)
            (else
              (Game|Damage|ApplyDamage Other _damage 0 0)
              (Audio|PlaySoundatLocation "/Game/PrototypeWeap/Sound/GrenadeLauncher/GL_Explosion06.GL_Explosion06" HitLocation "0, 0, 0" 1.0 1.0 0.0 0 0 0)))
          (Effects|SpawnEmitteratLocation (Variables|Default|GethitVFX) HitLocation)
          (Actor|DestroyActor) ; Then destroy this projectile
        )))))

(fn ConstructionScript)