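; Pistol Blueprint that fires player projectiles when its Shoot event is called.
; Shoot spawns a Player_projectile_BP at the AimArrow's world transform and plays the ShootEffect emitter at the same location and rotation.
; A debug line along the aim direction, scaled by Range, is left disconnected and never runs.
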(event EventBeginPlay)

(event Collision|EventActorBeginOverlap
  (params (OtherActor :type Actor%20Object%20Reference)))

(event EventTick
  (params (DeltaSeconds :type Float%20%28single-precision%29)))

(event EventShoot
  (bind _aimarrow (Variables|Default|GetaimArrow))
  (Game|SpawnActorfromClass "/Game/Blueprints/Player_projectile_BP.Player_projectile_BP_C" (Transformation|GetWorldTransform _aimarrow) "Undefined" 0 0)
  (Effects|SpawnEmitteratLocation (Variables|Default|GetshootEffect) (Transformation|GetWorldLocation _aimarrow) (Transformation|GetWorldRotation _aimarrow)))

(fn ConstructionScript)